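; Behavior tree task that makes an AI-controlled enemy fire a single shot at the player.
; On execute it spawns a BulletClass actor at the pawn's location, rotated toward player character 0, with the pawn as owner and instigator, and plays an attack sound.
; It finishes successfully after the shot, or fails if the pawn or player is invalid.
; The GetTargetActor blackboard lookup is disconnected, so TargetObject does not affect aim.
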(event `self.ReceiveTickAI`
  (params (OwnerController :type "AIController Object Reference") (ControlledPawn :type "Pawn Object Reference") (DeltaSeconds :type "Float (single-precision)")))

(event `Fire`)

(event `self.ReceiveExecuteAI`
  (params (OwnerController :type "AIController Object Reference") (ControlledPawn :type "Pawn Object Reference"))
  (bind _returnvalue (`GameplayStatics.GetPlayerCharacter` 0))
  (bind _returnvalue_2 (`Actor.K2_GetActorLocation` ControlledPawn))
  (`/Engine/EditorBlueprintResources/StandardMacros.IsValid` ControlledPawn
    (:`Is Valid`
      (`/Engine/EditorBlueprintResources/StandardMacros.IsValid` _returnvalue
        (:`Is Valid`
          (`|SpawnActorFromClass` (`self.BulletClass`) (`KismetMathLibrary.MakeTransform` _returnvalue_2 (`KismetMathLibrary.MakeRotFromX` (- (`Actor.K2_GetActorLocation` _returnvalue) _returnvalue_2))) "Undefined" "OverrideRootScale" ControlledPawn null ControlledPawn)
          (`GameplayStatics.SpawnSoundAtLocation` "/Game/Audio/Enemies/Enemy_attacknew_03_Cue.Enemy_attacknew_03_Cue" _returnvalue_2 (struct) 1.0 1.0 0.0 null null)
          (`self.FinishExecute` true))
        (:`Is Not Valid`
          (`self.FinishExecute` false :!label _label))))
    (:`Is Not Valid`
      (goto _label))))