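; Player inventory component that holds references to actors in a list capped by InventorySize.
; Adding stores the actor uniquely, binds to its destroyed event and fires OnActorAddedToInventory, with a destroy handler that removes the actor from the list.
; Removal fires no dispatcher and leaves the destroy binding in place.
; Add, remove and contains checks return success booleans and print debug messages, and a getter reports the item count.
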(fn `AddToInventory`
  (params (ActorToAdd :type "Actor Object Reference"))
  (returns (Added :type Boolean))
  (if (< (`KismetArrayLibrary.Array_Length` (`self.InventoryActors`)) (`self.InventorySize`))
    (`KismetArrayLibrary.Array_AddUnique` (`self.InventoryActors`) ActorToAdd)
    (`KismetSystemLibrary.PrintString` (`KismetStringLibrary.Concat_StrStr` "Added (" (`KismetTextLibrary.Conv_TextToString` (`KismetTextLibrary.Conv_StringToText` (`KismetSystemLibrary.GetDisplayName` ActorToAdd))) ") to inventory"))
    (add `Actor.OnDestroyed` ActorToAdd (`|CreateDelegate` :!event `OnInventoryItemDestroyed`))
    (`self.OnActorAddedToInventory` ActorToAdd)
    (return true)
    (else
      (`KismetSystemLibrary.PrintString` (`KismetStringLibrary.Concat_StrStr` "Failed to add (" (`KismetTextLibrary.Conv_TextToString` (`KismetTextLibrary.Conv_StringToText` (`KismetSystemLibrary.GetDisplayName` null))) ") to inventory, inventory is full"))
      (return false))))

(fn `GetNumItems`
  (returns (Size :type Integer))
  (return (`KismetArrayLibrary.Array_Length` (`self.InventoryActors`))))

(fn `InventoryContains`
  (params (Actor :type "Actor Object Reference"))
  (returns (ContainsActor :type Boolean))
  (if (`KismetArrayLibrary.Array_Contains` (`self.InventoryActors`) Actor)
    (`KismetSystemLibrary.PrintString` (`KismetStringLibrary.Concat_StrStr` "Inventory contains" (`KismetTextLibrary.Conv_TextToString` (`KismetTextLibrary.Conv_StringToText` (`KismetSystemLibrary.GetDisplayName` Actor)))))
    (return true)
    (else
      (`KismetSystemLibrary.PrintString` (`KismetStringLibrary.Concat_StrStr` "Inventory does not contain: " (`KismetTextLibrary.Conv_TextToString` (`KismetTextLibrary.Conv_StringToText` (`KismetSystemLibrary.GetDisplayName` Actor)))))
      (return false))))

(fn `OnInventoryItemDestroyed`
  (params (Actor :type "Actor Object Reference"))
  (`self.RemoveFromInventory` Actor))

(fn `RemoveFromInventory`
  (params (ActorToRemove :type "Actor Object Reference"))
  (returns (Removed :type Boolean))
  (bind _inventoryactors (`self.InventoryActors`))
  (if (`KismetArrayLibrary.Array_Contains` _inventoryactors ActorToRemove)
    (bind _returnvalue (`KismetArrayLibrary.Array_RemoveItem` _inventoryactors ActorToRemove))
    (if _returnvalue
      (`KismetSystemLibrary.PrintString` (`KismetStringLibrary.Concat_StrStr` "Removed (" (`KismetTextLibrary.Conv_TextToString` (`KismetTextLibrary.Conv_StringToText` (`KismetSystemLibrary.GetDisplayName` ActorToRemove))) ") from inventory"))
      (return true)
      (else
        (`KismetSystemLibrary.PrintString` (`KismetStringLibrary.Concat_StrStr` "Failed to remove (" (`KismetTextLibrary.Conv_TextToString` (`KismetTextLibrary.Conv_StringToText` (`KismetSystemLibrary.GetDisplayName` ActorToRemove))) ") from inventory"))
        (return false)))
    (else
      (`KismetSystemLibrary.PrintString` (`KismetStringLibrary.Concat_StrStr` "Failed to remove (" (`KismetTextLibrary.Conv_TextToString` (`KismetTextLibrary.Conv_StringToText` (`KismetSystemLibrary.GetDisplayName` ActorToRemove))) ") from inventory - not here"))
      (return false))))