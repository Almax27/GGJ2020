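; Player character for a twin-stick shooter, drawn as a Paper2D flipbook sprite with an attached weapon.
; While alive, Tick turns camera-relative stick input into movement, aim, auto-fire, a traced aim beam and sprite animation with footsteps; firing requires an empty inventory.
; CombatComponent death notifies the game mode after a delay, and damage plays a tint-and-shake timeline.
; A button triggers a voice emote with a temporary Beep_Boop actor, alongside debug damage and kill keys.
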(event `self.ReceiveBeginPlay`
  ;[1 1 1] Begin Play
  (add `/Game/Blueprints/Combat/CombatComponent.OnDeath` (`self.CombatComponent`) (`|CreateDelegate` :!event `OnDeath`))
  (bind _returnvalue (`|SpawnActorFromClass` (`self.DefaultWeapon`) (`self.GetTransform`) "Undefined" "OverrideRootScale" self self))
  (bind _output_get (set `self.ActiveWeapon` _returnvalue))
  (`/Engine/EditorBlueprintResources/StandardMacros.IsValid` _output_get
    (:`Is Valid`
      (`self.K2_AttachToComponent` _output_get (`self.WeaponSlot`) "None" "SnapToTarget" "SnapToTarget" "KeepRelative" true)
      (bind _returnvalue_2 (`PrimitiveComponent.CreateDynamicMaterialInstance` (`self.Sprite`) 0 (`PrimitiveComponent.GetMaterial` (`self.Sprite`) 0) "None"))
      (set `self.DynamicMaterial` _returnvalue_2))))

(event `OnDeath`
  (params (CombatComponent :type "/Game/Blueprints/Combat/CombatComponent Object Reference"))
  ;[1 1 1] Death
  (`WidgetBlueprintLibrary.SetInputMode_UIOnlyEx` (`GameplayStatics.GetPlayerController` 0) null)
  (`MovementComponent.StopMovementImmediately` (`self.CharacterMovement`))
  (`PaperFlipbookComponent.SetFlipbook` (`self.Sprite`) (`self.DeathFlipbook`))
  (`GameplayStatics.PlaySound2D` "/Game/Audio/Music/deathsting_Cue.deathsting_Cue" 1.0 1.0 0.0 null null)
  (`KismetSystemLibrary.Delay` 2.0)
  (bind _asgame_mode_bp (cast `/Game/Blueprints/GameModeBP` (`GameplayStatics.GetGameMode`)))
  (`/Game/Blueprints/GameModeBP.OnPlayerDeath` _asgame_mode_bp))

(event `self.ReceiveDestroyed`
  (bind _activeweapon (`self.ActiveWeapon`))
  (`/Engine/EditorBlueprintResources/StandardMacros.IsValid` _activeweapon
    (:`Is Valid`
      (`self.K2_DestroyActor` _activeweapon))))

(event `InputAction|Fire`
  (params (Key :type "Key Structure"))
  ;[1 1 1] Fire input
  (:`Pressed`
    (set `self.WantsToFire` true))
  (:`Released`
    (set `self.WantsToFire` false)))

(event `self.ReceiveTick`
  (params (DeltaSeconds :type "Float (single-precision)"))
  (bind _activeweapon (`self.ActiveWeapon`))
  (bind _wasgamecompleted (`/Game/Blueprints/GameInstanceBP.WasGameCompleted` (cast `/Game/Blueprints/GameInstanceBP` (`GameplayStatics.GetGameInstance`) :!pure true)))
  ;[1 1 1] Tick
  (if (and (`/Game/Blueprints/Combat/CombatComponent.IsAlive` (`self.CombatComponent`)) (not _wasgamecompleted))
    (`|ExecutionSequence`
      (:`then_0`
        (`self.TickInput`)
        (`self.TickAnimation`))
      (:`then_1`
        (`/Engine/EditorBlueprintResources/StandardMacros.IsValid` _activeweapon
          (:`Is Valid`
            (`/Game/Blueprints/Combat/BaseWeapon.SetIsAttacking` _activeweapon (and (`self.WantsToFire`) (`self.CanFire`)))
            (`self.K2_SetActorRotation` _activeweapon (`KismetMathLibrary.MakeRotFromX` (`self.AimDir`)) false))))
      (:`then_2`
        (`/Engine/EditorBlueprintResources/StandardMacros.IsValid` (stale `Key|Gamepad_FaceButton_Top` _returnvalue_2)
          (:`Is Valid`
            (`SceneComponent.K2_SetWorldLocation` (`Actor.RootComponent` (stale `Key|Gamepad_FaceButton_Top` _returnvalue_2)) (`SceneComponent.K2_GetComponentLocation` (`self.Sprite`)) false false)))))
    (elif _wasgamecompleted
      (`PaperFlipbookComponent.SetFlipbook` (`self.Sprite`) (`self.IdleFlipbook`)))))

(event `Key|Gamepad_FaceButton_Top`
  (params (Key :type "Key Structure"))
  (bind _sprite (`self.Sprite`))
  (bind _returnvalue (`SceneComponent.K2_GetComponentToWorld` _sprite))
  (:`Pressed`
    (`GameplayStatics.SpawnSoundAttached` "/Game/Audio/Robovoice/Robo_Voice.Robo_Voice" _sprite "None" (0.0 0.0 0.0) (struct) "KeepRelativeOffset" false 1.0 1.0 0.0 null null :!label _label)
    (`/Engine/EditorBlueprintResources/StandardMacros.DoOnce` false :!label _label_2
      (:`Completed`
        (bind _returnvalue_2 (`|SpawnActorFromClass` "/Game/Blueprints/Player/Beep_Boop.Beep_Boop_C" (`KismetMathLibrary.MakeTransform` (.location _returnvalue) (`KismetMathLibrary.MakeRotator` 45.0 45.0 (.yaw (.rotation _returnvalue))) (.scale _returnvalue)) "Undefined" "OverrideRootScale" null null))
        (`/Engine/EditorBlueprintResources/StandardMacros.IsValid` _returnvalue_2
          (:`Is Valid`
            (`KismetSystemLibrary.Delay` 1.0)
            (`self.K2_DestroyActor` _returnvalue_2)
            (goto _label_2 :!via `Reset`)))))))

(event `Key|E`
  (params (Key :type "Key Structure"))
  (:`Pressed`
    (goto _label)))

(event `Key|H`
  (params (Key :type "Key Structure"))
  ;[1 1 1] Debug
  (:`Pressed`
    (`self.ExecDebug`
      (:`Out`
        (`GameplayStatics.ApplyDamage` self 10.0 (`self.GetController`) self)))))

(event `Key|K`
  (params (Key :type "Key Structure"))
  ;[1 1 1] Debug
  (:`Pressed`
    (`self.ExecDebug`
      (:`Out`
        (`/Game/Blueprints/Combat/CombatComponent.Kill` (`self.CombatComponent`))))))

(event `TickAnimation`
  (bind _returnvalue (`self.GetInputAxisValue`))
  (bind _sprite (`self.Sprite`))
  (bind _returnvalue_2 (`PaperFlipbookComponent.GetPlaybackPositionInFrames` (`self.Sprite`)))
  ;[1 1 1] Animation
  (`|ExecutionSequence`
    (:`then_0`
      ;[1 1 1] Select flipbook
      (bind _returnvalue_3 (`PaperFlipbookComponent.SetFlipbook` (`self.Sprite`) (select `bool` (`/Game/Blueprints/Combat/CombatComponent.IsAlive` (`self.CombatComponent`)) :`false` (`self.DeathFlipbook`) :`true` (select `bool` (< (`/Game/Blueprints/Combat/CombatComponent.GetTimeSinceLastHit` (`self.CombatComponent`)) 0.3) :`false` (select `bool` (> (`KismetMathLibrary.VSizeXY` (`self.GetVelocity`)) 100.0) :`false` (`self.IdleFlipbook`) :`true` (`self.WalkFlipbook`)) :`true` (`self.HitFlipbook`)))))
      (if _returnvalue_3
        (`PaperFlipbookComponent.SetLooping` _sprite true)
        (`PaperFlipbookComponent.Play` _sprite)))
    (:`then_1`
      ;[1 1 1] Select  facing
      (if (!= (`KismetMathLibrary.VSizeXYSquared` (`self.AimDir`)) 0.0)
        (`SceneComponent.SetRelativeScale3D` (`self.Sprite`) (`KismetMathLibrary.MakeVector` (select `bool` (> (`self.GetInputAxisValue`) 0.0) :`false` 1.0 :`true` -1.0 :!type "Float (single-precision)") 1.0 1.0))
        (elif (and (!= (`KismetMathLibrary.VSizeXYSquared` (`self.MoveDir`)) 0.0) (> (`KismetMathLibrary.Abs` _returnvalue) -0.1))
          (`SceneComponent.SetRelativeScale3D` (`self.Sprite`) (`KismetMathLibrary.MakeVector` (select `bool` (> _returnvalue 0.0) :`false` 1.0 :`true` -1.0 :!type "Float (single-precision)") 1.0 1.0)))))
    (:`then_3`
      ;[1 1 1] Detect footsteps
      (if (> (`KismetMathLibrary.VSizeXYSquared` (`self.MoveDir`)) 0.0)
        (`|ExecutionSequence`
          (:`then_0`
            (if (and (== _returnvalue_2 0) (!= (`self.LastWalkFrame`) 0))
              (`/Engine/EditorBlueprintResources/StandardMacros.DoOnce` false :!label _label_3
                (:`Completed`
                  (`self.Footstep`)
                  (`KismetSystemLibrary.Delay` (* (`PaperFlipbook.GetTotalDuration` (`self.WalkFlipbook`)) 0.5))
                  (goto _label_3 :!via `Reset`)))))
          (:`then_1`
            (set `self.LastWalkFrame` _returnvalue_2)))))))

(event `Footstep`
  ;[1 1 1] Footsteps
  (`GameplayStatics.SpawnSoundAttached` "/Game/Audio/Footsteps/MainPlayer_Footsteps_00_Cue.MainPlayer_Footsteps_00_Cue" (`self.CapsuleComponent`) "None" (0.0 0.0 0.0) (struct) "KeepRelativeOffset" false 1.0 1.0 0.0 null null))

(event `self.ReceiveAnyDamage`
  (params (Damage :type "Float (single-precision)") (DamageType :type "DamageType Object Reference") (InstigatedBy :type "Controller Object Reference") (DamageCauser :type "Actor Object Reference"))
  (bind (_direction _shake _tint) (`Timeline|DamageReaction` :!via `PlayFromStart`)
    (:`Update`
      (`MaterialInstanceDynamic.SetVectorParameterValue` (`self.DynamicMaterial`) "Tint" _tint)
      (`SceneComponent.K2_SetRelativeLocation` (`self.Sprite`) (`KismetMathLibrary.MakeVector` (* _shake 30.0) (* _shake 30.0)) false false))
    (:`Finished`
      (`MaterialInstanceDynamic.SetVectorParameterValue` (`self.DynamicMaterial`) "Tint" (struct :`R` 1.0 :`G` 1.0 :`B` 1.0 :`A` 1.0))
      (`SceneComponent.K2_SetRelativeLocation` (`self.Sprite`) (0.0 0.0 0.0) false false))))

(fn `CanFire`
  (returns (CanFire :type Boolean))
  (bind _returnvalue (`self.GetComponentByClass` (`self.GetController`) "/Game/Blueprints/Player/InventoryComponent.InventoryComponent_C"))
  (`/Engine/EditorBlueprintResources/StandardMacros.IsValid` _returnvalue
    (:`Is Valid`
      (return (== (`/Game/Blueprints/Player/InventoryComponent.GetNumItems` _returnvalue) 0)))
    (:`Is Not Valid`
      (return true))))

(fn `TickInput`
  (locals (CameraRot :type "Rotator Structure"))
  (bind _returnvalue (`self.K2_GetActorLocation`))
  (bind _particlesystem (`self.ParticleSystem`))
  (bind _returnvalue_2 (`KismetMathLibrary.MakeVector` (`self.GetInputAxisValue`) (`self.GetInputAxisValue`)))
  (bind _returnvalue_3 (`KismetMathLibrary.MakeVector` (`self.GetInputAxisValue`) (`self.GetInputAxisValue`)))
  (bind _returnvalue_4 (`KismetMathLibrary.VSizeXY` _returnvalue_3))
  (bind _returnvalue_5 (+ _returnvalue (* (`KismetMathLibrary.Vector_Normal2D` (`self.AimDir`)) 5000.0)))
  (`|ExecutionSequence`
    (:`then_0`
      (set `local.CameraRot` (`KismetMathLibrary.MakeRotator` 0.0 0.0 (.yaw (`PlayerCameraManager.GetCameraRotation` (`GameplayStatics.GetPlayerCameraManager` 0))))))
    (:`then_1`
      ;[1 1 1] Move Input
      (if (> _returnvalue_4 (`self.MoveDeadzone`))
        (bind _output_get (set `self.MoveDir` (`KismetMathLibrary.GreaterGreater_VectorRotator` (`KismetMathLibrary.Normal` _returnvalue_3) (`local.CameraRot`))))
        (`self.AddMovementInput` _output_get _returnvalue_4)
        (else
          (set `self.MoveDir` (0.0 0.0 0.0)))))
    (:`then_2`
      ;[1 1 1] Aim Input
      (if (> (`KismetMathLibrary.VSizeXY` _returnvalue_2) (`self.AimDeadzone`))
        (set `self.AimDir` (`KismetMathLibrary.NegateVector` (`KismetMathLibrary.LessLess_VectorRotator` (`KismetMathLibrary.Normal` _returnvalue_2) (`local.CameraRot`))))
        (set `self.WantsToFire` true)
        (else
          (set `self.AimDir` (0.0 0.0 0.0))
          (set `self.WantsToFire` false))))
    (:`then_3`
      (if (and (`self.CanFire`) (> (`KismetMathLibrary.VSizeSquared` (`self.AimDir`)) 0.0))
        (`SceneComponent.SetVisibility` _particlesystem true false)
        (bind (_outhit _returnvalue_6) (`KismetSystemLibrary.LineTraceSingleByProfile` _returnvalue _returnvalue_5 "Bullet" true))
        (if _returnvalue_6
          (bind (_bblockinghit _binitialoverlap _time _distance _location _impactpoint) (`GameplayStatics.BreakHitResult` _outhit))
          (`ParticleSystemComponent.SetBeamTargetPoint` _particlesystem 0 _impactpoint 0)
          (`FXSystemComponent.SetVectorParameter` _particlesystem "Target" _impactpoint)
          (else
            (`ParticleSystemComponent.SetBeamTargetPoint` _particlesystem 0 _returnvalue_5 0)
            (`FXSystemComponent.SetVectorParameter` _particlesystem "Target" _returnvalue_5)))
        (else
          (`SceneComponent.SetVisibility` _particlesystem false false))))))

(fn `UserConstructionScript`)