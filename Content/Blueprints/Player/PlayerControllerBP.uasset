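; Player controller that manages the HUD, audio listener, interaction and item pickup for the possessed pawn.
; Each tick it selects an active interactable from a registered list by intended proximity, though the changed-target prompt logic is disconnected.
; Input triggers interaction or moves pickups between InventoryComponent and the pawn's flipbook, updating game mode flags.
; Debug-gated keys destroy all enemies or complete the game.
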(event `self.ReceivePossess`
  (params (PossessedPawn :type "Pawn Object Reference"))
  (`self.SetAudioListenerAttenuationOverride` (`Actor.RootComponent` PossessedPawn))
  (bind _returnvalue (`|CreateWidget` "/Game/Blueprints/UI/PlayerHUD.PlayerHUD_C" self))
  (bind _output_get (set `self.HUDRoot` _returnvalue))
  (`UserWidget.AddToViewport` _output_get 0))

(event `self.ReceiveUnPossess`
  (params (UnpossessedPawn :type "Pawn Object Reference"))
  (`self.ClearAudioListenerAttenuationOverride`)
  (`Widget.RemoveFromParent` (`self.HUDRoot`)))

(event `self.ReceiveBeginPlay`
  (add `/Game/Blueprints/Player/InventoryComponent.OnActorAddedToInventory` (`self.InventoryComponent`) (delegate `OnActorAddedToInventoryEvent`)))

(event `OnActorAddedToInventoryEvent`
  (params (NewActor :type "Actor Object Reference"))
  (bind _aspickup_actor_bp (cast `/Game/Blueprints/World/Interactable/PickupActorBP` NewActor))
  (switch `/Game/Blueprints/World/Interactable/PickupFlags` (`/Game/Blueprints/World/Interactable/PickupActorBP.PickupFlag` _aspickup_actor_bp)
    (:`NewEnumerator1`
      (`/Game/Blueprints/GameHelperFunctions.SetGameModeFlag` "NewEnumerator0" true))
    (:`NewEnumerator2`
      (`/Game/Blueprints/GameHelperFunctions.SetGameModeFlag` "NewEnumerator14"))))

(event `self.ReceiveTick`
  (params (DeltaSeconds :type "Float (single-precision)"))
  (`self.UpdateActiveInteractable`))

(event `InputAction|Pickup`
  (params (Key :type "Key Structure"))
  (:`Pressed`
    (bind _canpickup (`self.CanPickupInteractable`))
    (if _canpickup
      (`self.Pickup`)
      (else
        (`self.CanDropPickup`)
        (`self.Drop`)))))

(event `InputAction|Interact`
  (params (Key :type "Key Structure"))
  (bind _activeinteractable (`self.ActiveInteractable`))
  (:`Pressed`
    (`/Engine/EditorBlueprintResources/StandardMacros.IsValid` _activeinteractable
      (:`Is Valid`
        (if (`/Game/Blueprints/World/Interactable/BaseInteractable.IsInteractable` _activeinteractable)
          (`/Game/Blueprints/World/Interactable/BaseInteractable.Interact` (`self.ActiveInteractable`)))))))

(event `Key|BackSpace`
  (params (Key :type "Key Structure"))
  (:`Pressed`
    (`self.ExecDebug`
      (:`Out`
        (bind _outactors (`GameplayStatics.GetAllActorsOfClass` "/Game/Blueprints/Enemy/BaseEnemyCharacter.BaseEnemyCharacter_C"))
        (for _array_element _outactors
          (`self.K2_DestroyActor` _array_element))))))

(event `Key|C`
  (params (Key :type "Key Structure"))
  (:`Pressed`
    (`self.ExecDebug`
      (:`Out`
        (bind _asgame_mode_bp (cast `/Game/Blueprints/GameModeBP` (`GameplayStatics.GetGameMode`)))
        (`/Game/Blueprints/GameModeBP.CompleteGame` _asgame_mode_bp)))))

(fn `CanDropPickup`
  (returns (CanDrop :type Boolean))
  (for _array_element (`/Game/Blueprints/Player/InventoryComponent.InventoryActors` (`self.InventoryComponent`))
    (bind _aspickup_actor_bp (cast `/Game/Blueprints/World/Interactable/PickupActorBP` _array_element))
    (if (`/Game/Blueprints/World/Interactable/PickupActorBP.PickedUp` _aspickup_actor_bp)
      (return true)
      (else
        (return false))))
  (return false))

(fn `CanPickupInteractable`
  (returns (CanPickup :type Boolean))
  ;[1 1 1] Is Active Interactable a Pickup?
  (bind _asinteractable_pickup_bp (cast `/Game/Blueprints/World/Interactable/Interactable_PickupBP` (`self.ActiveInteractable`))
    (:`then`
      ;[1 1 1] Do I already have this pickup?
      (bind _containsactor (`/Game/Blueprints/Player/InventoryComponent.InventoryContains` (`self.InventoryComponent`) (`self.GetOwner` _asinteractable_pickup_bp)))
      (return (not _containsactor)))
    (:`CastFailed`
      (return false))))

(fn `DeregisterInteractable`
  (params (Intreractable :type "/Game/Blueprints/World/Interactable/BaseInteractable Object Reference"))
  (`/Engine/EditorBlueprintResources/StandardMacros.IsValid` Intreractable
    (:`Is Valid`
      (bind _returnvalue (`KismetArrayLibrary.Array_RemoveItem` (`self.RegisteredInteractables`) Intreractable))
      (if _returnvalue
        (set `/Game/Blueprints/World/Interactable/BaseInteractable.RegisteredTo` null Intreractable)
        (`KismetSystemLibrary.PrintString` (`KismetStringLibrary.Concat_StrStr` "Deregistered interactable:" (`KismetSystemLibrary.GetDisplayName` Intreractable)))))))

(fn `Drop`
  (for _array_element (`/Game/Blueprints/Player/InventoryComponent.InventoryActors` (`self.InventoryComponent`))
    (bind _aspickup_actor_bp (cast `/Game/Blueprints/World/Interactable/PickupActorBP` _array_element))
    (if (`/Game/Blueprints/World/Interactable/PickupActorBP.PickedUp` _aspickup_actor_bp)
      ;[1 1 1] Remove from inventory
      (bind _removed (`/Game/Blueprints/Player/InventoryComponent.RemoveFromInventory` (`self.InventoryComponent`) _aspickup_actor_bp))
      (if _removed
        (`self.K2_DetachFromActor` _aspickup_actor_bp "KeepWorld" "KeepRelative" "KeepRelative")
        (`/Game/Blueprints/World/Interactable/PickupActorBP.OnDropped` _aspickup_actor_bp)
        (`/Game/Blueprints/GameHelperFunctions.SetGameModeFlag` "NewEnumerator4")))))

(fn `Interact`)

(fn `OnActiveInteractableChanged`
  (params (Old :type "/Game/Blueprints/World/Interactable/BaseInteractable Object Reference") (New :type "/Game/Blueprints/World/Interactable/BaseInteractable Object Reference"))
  (locals (TextToDisplay :type Text)))

(fn `Pickup`
  (bind _rootcomponent (`Actor.RootComponent` (`self.K2_GetPawn`)))
  (bind _asinteractable_pickup_bp (cast `/Game/Blueprints/World/Interactable/Interactable_PickupBP` (`self.ActiveInteractable`)))
  (bind _associatedpickup (`/Game/Blueprints/World/Interactable/Interactable_PickupBP.AssociatedPickup` _asinteractable_pickup_bp))
  ;[1 1 1] Add pickup to inventory
  (bind _added (`/Game/Blueprints/Player/InventoryComponent.AddToInventory` (`self.InventoryComponent`) _associatedpickup))
  (if _added
    ;[1 1 1] Should no longer be in my registered interactables
    (`self.DeregisterInteractable` (`self.ActiveInteractable`))
    (`self.UpdateActiveInteractable`)
    ;[1 1 1] Notify pickup and attach to pawn
    (`self.K2_AttachToComponent` _associatedpickup (`self.GetComponentByClass` (`self.K2_GetPawn`) "/Script/Paper2D.PaperFlipbookComponent") "None" "SnapToTarget" "KeepRelative" "KeepRelative" true)
    (`/Game/Blueprints/World/Interactable/PickupActorBP.OnPickup` _associatedpickup)
    (`/Game/Blueprints/GameHelperFunctions.SetGameModeFlag` "NewEnumerator4" true)
    (`GameplayStatics.SpawnSoundAttached` "/Game/Audio/Footsteps/Pickup_Item.Pickup_Item" _rootcomponent "None" (0.0 0.0 0.0) (struct) "KeepRelativeOffset" false 1.0 1.0 0.0 null null)
    (`GameplayStatics.SpawnSoundAttached` "/Game/Audio/Robovoice/Robo_Voice.Robo_Voice" _rootcomponent "None" (0.0 0.0 0.0) (struct) "KeepRelativeOffset" false 1.0 1.0 0.0 null null)))

(fn `Register Interactable`
  (params (Interactable :type "/Game/Blueprints/World/Interactable/BaseInteractable Object Reference"))
  (set `/Game/Blueprints/World/Interactable/BaseInteractable.RegisteredTo` self Interactable)
  (`KismetArrayLibrary.Array_AddUnique` (`self.RegisteredInteractables`) Interactable)
  (`KismetSystemLibrary.PrintString` (`KismetStringLibrary.Concat_StrStr` "Registered Interactable:" (`KismetSystemLibrary.GetDisplayName` Interactable))))

(fn `UpdateActiveInteractable`
  (locals (ClosestDistance :type "Float (double-precision)") (ClosestInteractable :type "/Game/Blueprints/World/Interactable/BaseInteractable Object Reference"))
  (bind _registeredinteractables (`self.RegisteredInteractables`))
  (bind _closestdistance (`local.ClosestDistance`))
  (`KismetArrayLibrary.Array_RemoveItem` _registeredinteractables)
  (for _array_element _registeredinteractables
    (if (== (`local.ClosestDistance`) 0.0)
      (bind _returnvalue (`KismetMathLibrary.Vector_DistanceSquared` (`self.K2_GetActorLocation` _array_element) (`self.K2_GetActorLocation` (`self.K2_GetPawn`))))
      (set `local.ClosestDistance` _returnvalue)
      (set `local.ClosestInteractable` _array_element)
      (elif (< _returnvalue _closestdistance)
        (set `local.ClosestDistance` _closestdistance)
        (set `local.ClosestInteractable` _array_element))))
  (if (!= (`local.ClosestInteractable`) (`self.ActiveInteractable`))
    (`self.OnActiveInteractableChanged` (`self.ActiveInteractable`) (`local.ClosestInteractable`))
    (set `self.ActiveInteractable` (`local.ClosestInteractable`))))

(fn `UserConstructionScript`)