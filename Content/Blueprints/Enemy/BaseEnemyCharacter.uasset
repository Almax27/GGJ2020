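; Base enemy character, a flipbook sprite driven by a behavior tree, with a combat component and a health bar widget.
; Tick picks attack, hit, walk, idle or death flipbooks, mirroring the sprite relative to camera yaw toward the player when attacking, otherwise along its velocity.
; Damage plays a timeline tint and shake through a dynamic material and sprite offset.
; Death plays sounds, hides the health bar and destroys the actor after a delay.
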(event `self.ReceiveTick`
  (params (DeltaSeconds :type "Float (single-precision)"))
  (bind _returnvalue (`self.GetVelocity`))
  (bind _target (`self.GetBBTaget`))
  (bind _sprite (`self.Sprite`))
  (bind _sprite_2 (`self.Sprite`))
  (`|ExecutionSequence`
    (:`then_0`
      (if (`/Game/Blueprints/Combat/CombatComponent.IsAlive` (`self.CombatComponent`))
        (if (`self.GetIsAttacking`)
          (bind _returnvalue_2 (`PaperFlipbookComponent.SetFlipbook` _sprite (`self.AttackFlipbook`)))
          (if _returnvalue_2
            (`PaperFlipbookComponent.SetLooping` _sprite_2 false))
          (else
            (bind _returnvalue_3 (`PaperFlipbookComponent.SetFlipbook` _sprite (select `bool` (< (`/Game/Blueprints/Combat/CombatComponent.GetTimeSinceLastHit` (`self.CombatComponent`)) 0.3) :`false` (select `bool` (> (`KismetMathLibrary.VSizeXY` (`self.GetVelocity`)) 0.0) :`false` (`self.IdleFlipbook`) :`true` (`self.WalkFlipbook`)) :`true` (`self.HitFlipbook`))))
            (if _returnvalue_3
              (`PaperFlipbookComponent.SetLooping` _sprite_2 true)
              (`PaperFlipbookComponent.Play` _sprite_2))))
        (else
          (`PaperFlipbookComponent.SetFlipbook` (`self.Sprite`) (`self.DeathFlipbook`)))))
    (:`then_1`
      (if (`self.GetIsAttacking`)
        (`/Engine/EditorBlueprintResources/StandardMacros.IsValid` _target
          (:`Is Valid`
            (`self.LookAtLocation` (`self.K2_GetActorLocation` _target)))
          (:`Is Not Valid`
            (if (> (`KismetMathLibrary.VSizeXY` _returnvalue) 0.0) :!label _label
              (`self.LookAtLocation` (+ (`self.K2_GetActorLocation`) _returnvalue)))))
        (else
          (goto _label))))))

(event `self.ReceiveBeginPlay`
  (bind _sprite (`self.Sprite`))
  (add `/Game/Blueprints/Combat/CombatComponent.OnDeath` (`self.CombatComponent`) (delegate `OnDeath`))
  (bind _asaicontroller (cast `AIController` (`self.GetController`)))
  (`AIController.RunBehaviorTree` _asaicontroller (`self.Behaviour`))
  (bind _asenemy_healthbar_widget (cast `/Game/Blueprints/Enemy/EnemyHealthbarWidget` (`WidgetComponent.GetUserWidgetObject` (`self.HealthbarComponent`))))
  (set `/Game/Blueprints/Enemy/EnemyHealthbarWidget.OwningActor` self _asenemy_healthbar_widget)
  (`/Game/Blueprints/Enemy/EnemyHealthbarWidget.OnOwningActorSet_Event` _asenemy_healthbar_widget)
  (bind _returnvalue (`PrimitiveComponent.CreateDynamicMaterialInstance` _sprite 0 (`PrimitiveComponent.GetMaterial` _sprite 0) "None"))
  (set `self.DynamicMaterial` _returnvalue))

(event `OnDeath`
  (params (CombatComponent :type "/Game/Blueprints/Combat/CombatComponent Object Reference"))
  (bind _capsulecomponent (`self.CapsuleComponent`))
  (`GameplayStatics.SpawnSoundAttached` "/Game/Audio/Enemies/Enemy_Die_00_Cue.Enemy_Die_00_Cue" _capsulecomponent "None" (0.0 0.0 0.0) (struct) "KeepRelativeOffset" false 1.0 1.0 0.0 null null)
  (`GameplayStatics.SpawnSoundAttached` "/Game/Audio/Enemies/Enemy_Die_Vox_00_Cue.Enemy_Die_Vox_00_Cue" _capsulecomponent "None" (0.0 0.0 0.0) (struct) "KeepRelativeOffset" false 1.0 1.0 0.0 null null)
  (`SceneComponent.SetVisibility` (`self.HealthbarComponent`) false false)
  (`KismetSystemLibrary.Delay` 2.0)
  (`self.K2_DestroyActor`))

(event `self.ReceiveAnyDamage`
  (params (Damage :type "Float (single-precision)") (DamageType :type "DamageType Object Reference") (InstigatedBy :type "Controller Object Reference") (DamageCauser :type "Actor Object Reference"))
  (if (`/Game/Blueprints/Combat/CombatComponent.IsAlive` (`self.CombatComponent`))
    (bind (_direction _shake _tint) (`Timeline|Timeline_0` :!via `PlayFromStart`)
      (:`Update`
        (`MaterialInstanceDynamic.SetVectorParameterValue` (`self.DynamicMaterial`) "Tint" _tint)
        (`SceneComponent.K2_SetRelativeLocation` (`self.Sprite`) (`KismetMathLibrary.MakeVector` (* _shake 30.0) (* _shake 30.0)) false false))
      (:`Finished`
        (`MaterialInstanceDynamic.SetVectorParameterValue` (`self.DynamicMaterial`) "Tint" (struct :`R` 1.0 :`G` 1.0 :`B` 1.0 :`A` 1.0))
        (`SceneComponent.K2_SetRelativeLocation` (`self.Sprite`) (0.0 0.0 0.0) false false)))))

(fn `GetBBTaget`
  (returns (Target :type "Actor Object Reference"))
  (return (`GameplayStatics.GetPlayerCharacter` 0)))

(fn `GetIsAttacking`
  (returns (IsAttacking :type Boolean))
  (return (`BlackboardComponent.GetValueAsBool` (`AIBlueprintHelperLibrary.GetBlackboard` null) "IsAttacking")))

(fn `LookAtLocation`
  (params (Location :type "Vector Structure"))
  (`SceneComponent.SetRelativeScale3D` (`self.Sprite`) (`KismetMathLibrary.MakeVector` (select `bool` (> (.y (`KismetMathLibrary.LessLess_VectorRotator` (`KismetMathLibrary.Vector_Normal2D` (- Location (`self.K2_GetActorLocation`))) (`KismetMathLibrary.MakeRotator` 0.0 0.0 (.yaw (`PlayerCameraManager.GetCameraRotation` (`GameplayStatics.GetPlayerCameraManager` 0)))))) 0.0) :`false` 1.0 :`true` -1.0 :!type "Float (single-precision)") 1.0 1.0)))

(fn `UserConstructionScript`)