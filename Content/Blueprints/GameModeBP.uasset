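; Game mode that runs the game flow: title or respawn screen on begin play, death, room changes and completion.
; GameInstanceBP flags choose the opening screen and persist across the level reloads that follow the death and end screens.
; Entering a room blends the camera to that room actor and swaps the active room.
; Combat start and end pop and push a music sound mix, and completion fades the music out.
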(event `PresentWidget`)

(event `self.ReceiveBeginPlay`
  (bind _asgame_instance_bp (cast `/Game/Blueprints/GameInstanceBP` (`GameplayStatics.GetGameInstance`)))
  (if (or (`/Game/Blueprints/GameInstanceBP.IsFirstStart` _asgame_instance_bp) (`/Game/Blueprints/GameInstanceBP.WasGameCompleted` _asgame_instance_bp))
    (bind _returnvalue (`|CreateWidget` "/Game/Blueprints/UI/TitleScreen.TitleScreen_C" (`GameplayStatics.GetPlayerController` 0)))
    (`UserWidget.AddToViewport` _returnvalue 0)
    (else
      (`self.StartGame`)
      (bind _returnvalue_2 (`|CreateWidget` "/Game/Blueprints/UI/RespawnScreen.RespawnScreen_C" (`GameplayStatics.GetPlayerController` 0)))
      (`UserWidget.AddToViewport` _returnvalue_2 0))))

(event `StartGame`
  (`WidgetBlueprintLibrary.SetInputMode_GameOnly` (`GameplayStatics.GetPlayerController` 0))
  (bind _asgame_instance_bp (cast `/Game/Blueprints/GameInstanceBP` (`GameplayStatics.GetGameInstance`)))
  (set `/Game/Blueprints/GameInstanceBP.IsFirstStart` false _asgame_instance_bp)
  (set `/Game/Blueprints/GameInstanceBP.WasGameCompleted` false _asgame_instance_bp)
  (`self.Init Rooms`)
  (bind _main_theme (`self.InitMusic`)))

(event `OnPlayerDeath`
  ;[1 1 1] Death
  (bind _returnvalue (`|CreateWidget` "/Game/Blueprints/UI/DeathScreen.DeathScreen_C" (`GameplayStatics.GetPlayerController` 0)))
  (`UserWidget.AddToViewport` _returnvalue 0)
  (add `/Game/Blueprints/UI/DeathScreen.OnFadedIn` _returnvalue (delegate `OnDeathScreenFadedIn`))
  (`self.CombatEnded`))

(event `OnDeathScreenFadedIn`
  ;[1 1 1] Death
  (bind _returnvalue (`GameplayStatics.GetCurrentLevelName` true))
  (`GameplayStatics.OpenLevel` (`KismetStringLibrary.Conv_StringToName` _returnvalue)))

(event `OnRoomEntered`
  (params (Room :type "/Game/Blueprints/World/BaseRoom Object Reference"))
  (bind _activeroom (`self.ActiveRoom`))
  (`/Engine/EditorBlueprintResources/StandardMacros.IsValid` Room
    (:`Is Valid`
      (`|ExecutionSequence`
        (:`then_0`
          (`/Engine/EditorBlueprintResources/StandardMacros.IsValid` _activeroom
            (:`Is Valid`
              (`/Game/Blueprints/World/BaseRoom.OnPlayerLeft` _activeroom))))
        (:`then_1`
          (`PlayerController.SetViewTargetWithBlend` (`GameplayStatics.GetPlayerController` 0) Room (select `bool` (`KismetSystemLibrary.IsValid` (`self.ActiveRoom`)) :`true` 1.0 :!type "Float (single-precision)") "VTBlend_Cubic" 2.0 true))
        (:`then_2`
          (bind _output_get (set `self.ActiveRoom` Room))
          (`/Game/Blueprints/World/BaseRoom.OnPlayerEntered` _output_get))))))

(event `CompleteGame`
  (bind _asgame_instance_bp (cast `/Game/Blueprints/GameInstanceBP` (`GameplayStatics.GetGameInstance`)))
  (if (not (`/Game/Blueprints/GameInstanceBP.WasGameCompleted` _asgame_instance_bp))
    (`self.OnComplete`)
    (`AudioComponent.FadeOut` (stale `StartGame` _main_theme) 4.0 0.0 "Linear")
    (`|ExecutionSequence`
      (:`then_0`
        (set `/Game/Blueprints/GameInstanceBP.WasGameCompleted` true _asgame_instance_bp)
        (`WidgetBlueprintLibrary.SetInputMode_UIOnlyEx` (`GameplayStatics.GetPlayerController` 0) null)
        (`MovementComponent.StopMovementImmediately` (`Character.CharacterMovement` (`GameplayStatics.GetPlayerCharacter` 0)))
        (`KismetSystemLibrary.Delay` 2.0)
        (bind _returnvalue (`|CreateWidget` "/Game/Blueprints/UI/EndScreen.EndScreen_C" (`GameplayStatics.GetPlayerController` 0)))
        (`UserWidget.AddToViewport` _returnvalue 0)
        (add `/Game/Blueprints/UI/EndScreen.OnFinished` _returnvalue (delegate `OnEndScreenFinished`)))
      (:`then_1`
        (`KismetSystemLibrary.Delay` 3.0)
        (`GameplayStatics.PlaySound2D` "/Game/Audio/Ambience/ship_explosion.ship_explosion" 1.0 1.0 0.0 null null)))))

(event `OnEndScreenFinished`
  (bind _returnvalue (`GameplayStatics.GetCurrentLevelName` true))
  (`GameplayStatics.OpenLevel` (`KismetStringLibrary.Conv_StringToName` _returnvalue)))

(event `CombatStarted`
  (`GameplayStatics.PopSoundMixModifier` "/Game/Audio/Soundclass/Soundmix_Music.Soundmix_Music"))

(event `CombatEnded`
  (`GameplayStatics.PushSoundMixModifier` "/Game/Audio/Soundclass/Soundmix_Music.Soundmix_Music"))

(fn `Init Rooms`
  (bind _outactors (`GameplayStatics.GetAllActorsOfClass` "/Game/Blueprints/World/BaseRoom.BaseRoom_C"))
  (set `self.Rooms` _outactors))

(fn `InitMusic`
  (returns (`Main theme` :type "AudioComponent Object Reference"))
  (`GameplayStatics.PushSoundMixModifier` "/Game/Audio/Soundclass/Soundmix_Music.Soundmix_Music")
  (bind _returnvalue (`GameplayStatics.SpawnSound2D` "/Game/Audio/Music/asongiguess_loop.asongiguess_loop" 1.0 1.0 0.0 null))
  (return _returnvalue))

(fn `UserConstructionScript`)