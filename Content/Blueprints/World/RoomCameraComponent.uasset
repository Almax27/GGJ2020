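; RoomCameraComponent places a room's camera in the world when play begins.
; By default it takes a fixed isometric-style angle, pitched down and yawed diagonally, backed off from its owner's location by Distance along the view direction.
; If CopyTransformFrom is valid, it instead copies the world transform of that actor's RoomCameraComponent.
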(event `self.ReceiveBeginPlay`
  (`self.Setup`))

(event `Setup`
  (bind _returnvalue (`KismetMathLibrary.MakeRotator` 0.0 -45.0 45.0))
  (bind _copytransformfrom (`self.CopyTransformFrom`))
  (`/Engine/EditorBlueprintResources/StandardMacros.IsValid` _copytransformfrom
    (:`Is Valid`
      (`self.K2_SetWorldTransform` (`self.K2_GetComponentToWorld` (`Actor.GetComponentByClass` _copytransformfrom "RoomCameraComponent_C"))))
    (:`Is Not Valid`
      (`self.K2_SetWorldLocationAndRotation` (+ (`Actor.K2_GetActorLocation` (`self.GetOwner`)) (* (`KismetMathLibrary.NegateVector` (`KismetMathLibrary.GetForwardVector` _returnvalue)) (`self.Distance`))) _returnvalue))))