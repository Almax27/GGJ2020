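; A trigger actor that changes a configurable game mode flag when the player character overlaps it.
; On begin overlap it either toggles the flag's current state or sets it to a fixed value, with an Invert option that makes that value false instead of true.
; An optional clear on end overlap writes the opposite fixed value, regardless of whether entry toggled the flag.
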(event `self.ReceiveActorBeginOverlap`
  (params (OtherActor :type "Actor Object Reference"))
  (bind _flag (`self.Flag`))
  (cast `/Game/Blueprints/Player/PlayerCharacter` OtherActor)
  (if (`self.ToggleOnBeginOverlap`)
    (`/Game/Blueprints/GameHelperFunctions.SetGameModeFlag` _flag (not (`/Game/Blueprints/GameHelperFunctions.IsGameModeFlagSet` _flag)))
    (else
      (`/Game/Blueprints/GameHelperFunctions.SetGameModeFlag` _flag (not (`self.Invert`))))))

(event `self.ReceiveActorEndOverlap`
  (params (OtherActor :type "Actor Object Reference"))
  (cast `/Game/Blueprints/Player/PlayerCharacter` OtherActor)
  (if (`self.ClearOnEndOverlap`)
    (`/Game/Blueprints/GameHelperFunctions.SetGameModeFlag` (`self.Flag`) (`self.Invert`))))

(fn `UserConstructionScript`)