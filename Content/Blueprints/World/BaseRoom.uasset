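; BaseRoom is a room actor with its own RoomCamera that tells the game mode when the player enters.
; Actor overlaps with the player call OnRoomEntered on GameModeBP, while separate entered/left events track occupancy, with a camera pan sound on entry.
; BeginPlay and OnReset share a path that sets up the camera, clears occupancy and scans shape components for an already overlapping player.
; RoomHiderComponent visibility toggles are present but disconnected.
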(event `self.K2_OnReset`
  (`/Game/Blueprints/World/RoomCameraComponent.Setup` (`self.RoomCamera`) :!label _label)
  (`self.OnPlayerLeft`)
  (for _array_element (`self.K2_GetComponentsByClass` "/Script/Engine.ShapeComponent")
    (bind (_outactors _returnvalue) (`KismetSystemLibrary.ComponentOverlapActors` _array_element (`SceneComponent.K2_GetComponentToWorld` _array_element) (`|MakeArray` "ObjectTypeQuery3" :!type "EObjectTypeQuery Enum") "/Game/Blueprints/Player/PlayerCharacter.PlayerCharacter_C"))
    (if _returnvalue
      (`self.OnOverlapWithPlayer`)
      (break))))

(event `self.ReceiveBeginPlay`
  (goto _label))

(event `self.ReceiveActorBeginOverlap`
  (params (OtherActor :type "Actor Object Reference"))
  (cast `/Game/Blueprints/Player/PlayerCharacter` OtherActor)
  (`self.OnOverlapWithPlayer`))

(event `OnOverlapWithPlayer`
  (bind _asgame_mode_bp (cast `/Game/Blueprints/GameModeBP` (`GameplayStatics.GetGameMode`)))
  (`/Game/Blueprints/GameModeBP.OnRoomEntered` _asgame_mode_bp self))

(event `OnPlayerEntered`
  (set `self.IsPlayerInside` true)
  (`GameplayStatics.PlaySound2D` "/Game/Audio/Ambience/Camera_pan_Cue.Camera_pan_Cue" 1.0 1.0 0.0 null null))

(event `OnPlayerLeft`
  (set `self.IsPlayerInside` false))

(fn `UserConstructionScript`
  (`/Game/Blueprints/World/RoomCameraComponent.Setup` (`self.RoomCamera`)))