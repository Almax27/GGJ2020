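; Triggerable door that slides up once the player has overlapped it and its trigger condition is met.
; Player overlap latches WantsOpen, and game mode flag changes re-evaluate the door through RefreshDoor.
; RefreshDoor swaps the emissive material to show lock state, then plays or reverses a Timeline driving the mesh height.
; DoOnce-gated branches play open and close sounds, with opening fading out the ambient loop started at BeginPlay.
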(event `self.ReceiveBeginPlay`
  (`parent.ReceiveBeginPlay`)
  (`self.RefreshDoor`)
  (bind _returnvalue (`GameplayStatics.SpawnSoundAttached` "/Game/Audio/Ambience/AMB_Light_Loop_00_Cue.AMB_Light_Loop_00_Cue" (`self.Cube`) "None" (0.0 0.0 0.0) (struct) "KeepRelativeOffset" false 1.0 1.0 0.0 null null)))

(event `self.ReceiveActorBeginOverlap`
  (params (OtherActor :type "Actor Object Reference"))
  (`parent.ReceiveActorBeginOverlap` OtherActor)
  (cast `/Game/Blueprints/Player/PlayerCharacter` OtherActor)
  (set `self.WantsOpen` true)
  (`self.RefreshDoor`))

(event `self.OnGameModeFlagChangedEvent`
  (`self.RefreshDoor`))

(event `RefreshDoor`
  (`self.RefreshLockStatus`)
  (if (and (`self.WantsOpen`) (`self.CanBeTriggered`))
    (`|ExecutionSequence`
      (:`then_0`
        (bind (_direction _heightoffset) (`Timeline|Timeline_0` :!label _label)
          (:`Update`
            (`SceneComponent.K2_SetRelativeLocation` (`self.Cube`) (`KismetMathLibrary.MakeVector` 0.0 0.0 (* _heightoffset (`self.OpenedHeight`))) false false))))
      (:`then_1`
        (`/Engine/EditorBlueprintResources/StandardMacros.DoOnce` false
          (:`Completed`
            (`GameplayStatics.SpawnSoundAttached` "/Game/Audio/Interactables/Open_Door_Cue.Open_Door_Cue" (`self.Cube`) "None" (0.0 0.0 0.0) (struct) "KeepRelativeOffset" false 1.0 1.0 0.0 null null)
            (`KismetSystemLibrary.Delay` 0.5)
            (`GameplayStatics.SpawnSoundAttached` "/Game/Audio/Interactables/Door_Reached_Open_Cue.Door_Reached_Open_Cue" (`self.Cube`) "None" (0.0 0.0 0.0) (struct) "KeepRelativeOffset" false 1.0 1.0 0.0 null null)
            (`AudioComponent.FadeOut` (stale `self.ReceiveBeginPlay` _returnvalue) 0.4 0.0 "Linear")))))
    (else
      (`|ExecutionSequence`
        (:`then_0`
          (goto _label :!via `Reverse`))
        (:`then_1`
          (`/Engine/EditorBlueprintResources/StandardMacros.DoOnce` false
            (:`Completed`
              (`GameplayStatics.SpawnSoundAttached` "/Game/Audio/Interactables/Close_Door_Cue.Close_Door_Cue" (`self.Cube`) "None" (0.0 0.0 0.0) (struct) "KeepRelativeOffset" false 1.0 1.0 0.0 null null)
              (`KismetSystemLibrary.Delay` 0.5)
              (`GameplayStatics.SpawnSoundAttached` "/Game/Audio/Interactables/Door_Reached_Closed_Cue.Door_Reached_Closed_Cue" (`self.Cube`) "None" (0.0 0.0 0.0) (struct) "KeepRelativeOffset" false 1.0 1.0 0.0 null null))))))))

(event `RefreshLockStatus`
  (`PrimitiveComponent.SetMaterial` (`self.Cube`) 1 (select `bool` (`self.CanBeTriggered`) :`false` "/Game/Materials/Instances/Inst_DoorEm_Locked.Inst_DoorEm_Locked" :`true` "/Game/Materials/Instances/Inst_DoorEm.Inst_DoorEm" :!type "MaterialInterface Object Reference")))

(fn `UserConstructionScript`
  (`parent.UserConstructionScript`))