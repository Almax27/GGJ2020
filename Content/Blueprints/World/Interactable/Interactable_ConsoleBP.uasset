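; Interactable console that accepts a pickup actor brought into its overlap, recording progress through game mode flags.
; While interactable, it polls overlaps on Tick, snaps an unclaimed pickup to itself and sets the flag matching First or Second Pickup.
; A recognized pickup disables further interaction, updates the screen's dynamic material, fires the trigger and plays a lights-on cue if the second flag is set, otherwise a collect cue.
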(event `self.ReceiveTick`
  (params (DeltaSeconds :type "Float (single-precision)"))
  (`parent.ReceiveTick` DeltaSeconds)
  (if (`self.IsInteractable`)
    (for _array_element (`self.GetOverlappingActors` "/Game/Blueprints/World/Interactable/PickupActorBP.PickupActorBP_C")
      (bind _aspickup_actor_bp (cast `/Game/Blueprints/World/Interactable/PickupActorBP` _array_element))
      (if (not (`/Game/Blueprints/World/Interactable/PickupActorBP.PickedUp` _aspickup_actor_bp))
        (`self.K2_AttachToActor` _aspickup_actor_bp self "None" "SnapToTarget" "KeepWorld" "KeepRelative" true)
        (`/Game/Blueprints/World/Interactable/PickupActorBP.OnPickup` _aspickup_actor_bp)
        (switch `/Game/Blueprints/World/Interactable/PickupFlags` (`/Game/Blueprints/World/Interactable/PickupActorBP.PickupFlag` _aspickup_actor_bp)
          (:`NewEnumerator1`
            (`/Game/Blueprints/GameHelperFunctions.SetGameModeFlag` "NewEnumerator13" true))
          (:`NewEnumerator2`
            (`/Game/Blueprints/GameHelperFunctions.SetGameModeFlag` "NewEnumerator14" true)))
        (set `self.IsInteractable` false)
        (`MaterialInstanceDynamic.SetScalarParameterValue` (`self.DynamicMat`) "IsOnline" 0.5)
        (`/Game/Blueprints/World/Interactable/BaseTrigger.OnTrigger`)
        (if (`/Game/Blueprints/GameHelperFunctions.IsGameModeFlagSet` "NewEnumerator14")
          (`GameplayStatics.PlaySound2D` "/Game/Audio/Ambience/AMB_Turn_On_Lights_Cue.AMB_Turn_On_Lights_Cue" 1.0 1.0 0.0 null null)
          (else
            (`GameplayStatics.PlaySound2D` "/Game/Audio/UI/GGJ_Collect_Pickup_00_Cue.GGJ_Collect_Pickup_00_Cue" 1.0 1.0 0.0 null null)))))))

(fn `UserConstructionScript`
  (`parent.UserConstructionScript`)
  (bind _returnvalue (`PrimitiveComponent.CreateDynamicMaterialInstance` (`self.AnnouncementTv`) 1 "/Game/Materials/Masters/AnnouncementTV.AnnouncementTV" "None"))
  (set `self.DynamicMat` _returnvalue))