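; Base logic for a world pickup actor that can be carried and dropped, paired with a separately spawned interactable.
; On BeginPlay it spawns the interactable at its transform and links itself as the associated pickup.
; Pickup deletes the interactable, then shrinks and offsets the actor; dropping respawns it, restores scale and plays a sound.
; Dropping or destroying the actor clears its game mode flag, and destruction also removes the interactable.
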(event `self.ReceiveBeginPlay`
  (`self.SpawnInteractable`))

(event `self.ReceiveDestroyed`
  (bind _spawnedinteractable (`self.SpawnedInteractable`))
  (`/Game/Blueprints/GameHelperFunctions.SetGameModeFlag` (`self.PickupGameModeFlag`))
  (`/Engine/EditorBlueprintResources/StandardMacros.IsValid` _spawnedinteractable
    (:`Is Valid`
      (`self.K2_DestroyActor` _spawnedinteractable))))

(fn `Delete Interactable`
  (bind _spawnedinteractable (`self.SpawnedInteractable`))
  (if (`KismetSystemLibrary.IsValid` _spawnedinteractable)
    (`self.K2_DestroyActor` _spawnedinteractable)
    (set `self.SpawnedInteractable` null)))

(fn `OnDropped`
  (`self.SpawnInteractable`)
  (set `self.PickedUp` false)
  (`/Game/Blueprints/GameHelperFunctions.SetGameModeFlag` (`self.PickupGameModeFlag`))
  (`self.SetActorRelativeScale3D` (`KismetMathLibrary.Conv_DoubleToVector` 1.0))
  (`GameplayStatics.SpawnSoundAttached` "/Game/Audio/Footsteps/Drop_Item1.Drop_Item1" null "None" (0.0 0.0 0.0) (struct) "KeepRelativeOffset" false 1.0 1.0 0.0 null null))

(fn `OnPickup`
  (`self.Delete Interactable`)
  (set `self.PickedUp` true)
  (`self.SetActorRelativeScale3D` (`KismetMathLibrary.Conv_DoubleToVector` 0.5))
  (`self.K2_SetActorRelativeLocation` (50.0 -30.0 -20.0)))

(fn `SpawnInteractable`
  (bind _returnvalue (`|SpawnActorFromClass` (`self.InteractableToSpawn`) (`self.GetTransform` self) "AlwaysSpawn" "OverrideRootScale" self null))
  (bind _output_get (set `self.SpawnedInteractable` _returnvalue))
  (bind _asinteractable_pickup_bp (cast `/Game/Blueprints/World/Interactable/Interactable_PickupBP` _output_get))
  (set `/Game/Blueprints/World/Interactable/Interactable_PickupBP.AssociatedPickup` self _asinteractable_pickup_bp))

(fn `UserConstructionScript`)