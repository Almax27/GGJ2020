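; Wave-based enemy spawner that starts combat when triggered, optionally by player overlap.
; Each wave spawns its enemy classes at random intervals, cycling through shuffled actor-relative locations projected onto the navmesh.
; Destroyed-enemy callbacks advance to the next delayed wave once none remain alive, and the last sets a cleared flag and fires OnCleared.
; Combat start and end are reported to GameModeBP, and reset destroys active enemies and clears progress.
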(event `self.ReceiveBeginPlay`
  (if (not (> (`KismetArrayLibrary.Array_Length` (`self.SpawnLocations`)) 0))
    (`self.PrintDebug` " has no SpawnLocations set!! Adding ActorLocation as fallback..."
      (:`Out`
        (`KismetArrayLibrary.Array_Add` (`self.SpawnLocations`))))))

(event `self.ReceiveActorBeginOverlap`
  (params (OtherActor :type "Actor Object Reference"))
  (cast `/Game/Blueprints/Player/PlayerCharacter` OtherActor)
  (if (`self.SpawnOnPlayerEnter`)
    (`self.StartSpawning`)))

(event `self.K2_OnReset`
  (bind _activeenemies (`self.ActiveEnemies`))
  (`|ExecutionSequence`
    (:`then_0`
      (if (`self.HasStarted`)
        (bind _asgame_mode_bp (cast `/Game/Blueprints/GameModeBP` (`GameplayStatics.GetGameMode`)))
        (`/Game/Blueprints/GameModeBP.CombatEnded` _asgame_mode_bp)))
    (:`then_1`
      (set `self.WaveIndex` 0)
      (set `self.SpawnIndex` 0)
      (set `self.HasStarted` false)
      (`/Game/Blueprints/GameHelperFunctions.SetGameModeFlag` (`self.AllWavesClearedFlag`))
      (`/Game/Blueprints/GameHelperFunctions.SetGameModeFlag` (`self.ActiveFlag`))
      (`KismetSystemLibrary.K2_ClearAndInvalidateTimerHandle` (`self.NextSpawnTimer`)))
    (:`then_2`
      (for _array_element _activeenemies
        (`self.K2_DestroyActor` _array_element))
      (`KismetArrayLibrary.Array_Clear` _activeenemies))))

(event `StartSpawning`
  (if (not (`self.HasStarted`))
    (set `self.HasStarted` true)
    (`/Game/Blueprints/GameHelperFunctions.SetGameModeFlag` (`self.ActiveFlag`) true)
    (set `self.SpawnIndex` 0)
    (`KismetArrayLibrary.Array_Shuffle` (`self.SpawnLocations`))
    (`self.PrintDebug` "STARTED"
      (:`Out`
        (bind _asgame_mode_bp (cast `/Game/Blueprints/GameModeBP` (`GameplayStatics.GetGameMode`)))
        (`/Game/Blueprints/GameModeBP.CombatStarted` _asgame_mode_bp)
        (`self.SpawnNextEnemy`)
        (`self.CheckForClear`)))))

(event `CheckForClear`
  (if (and (`self.HasStarted`) (== (`KismetArrayLibrary.Array_Length` (`self.ActiveEnemies`)) 0))
    (bind _result (`/Engine/EditorBlueprintResources/StandardMacros.IncrementInt` (`self.WaveIndex`))
      (:`  `
        (if (>= _result (`KismetArrayLibrary.Array_Length` (`self.Waves`)))
          (`/Game/Blueprints/GameHelperFunctions.SetGameModeFlag` (`self.AllWavesClearedFlag`) true)
          (`self.OnCleared`)
          (`/Game/Blueprints/GameHelperFunctions.SetGameModeFlag` (`self.ActiveFlag`))
          (`self.PrintDebug` "COMPLETE"
            (:`Out`
              (bind _asgame_mode_bp (cast `/Game/Blueprints/GameModeBP` (`GameplayStatics.GetGameMode`)))
              (`/Game/Blueprints/GameModeBP.CombatEnded` _asgame_mode_bp)))
          (else
            (set `self.SpawnIndex` 0)
            (bind _returnvalue (`KismetSystemLibrary.K2_SetTimerDelegate` (`|CreateDelegate` :!event `SpawnNextEnemy`) (`.StartDelay_16_DAFDB201401CC823AAD5A3AFF0B9B9B4` (break `/Game/Blueprints/World/EnemyWaveDef` (`|GetArrayItem` (`self.Waves`) (`self.WaveIndex`))))))
            (set `self.NextSpawnTimer` _returnvalue)))))))

(event `SpawnNextEnemy`
  (bind _waves (`self.Waves`))
  (bind _waveindex (`self.WaveIndex`))
  (bind _spawnindex (`self.SpawnIndex`))
  (bind _spawnlocations (`self.SpawnLocations`))
  (bind (_enemiesinwave _startdelay _minspawninterval _maxspawninterval) (break `/Game/Blueprints/World/EnemyWaveDef` (`|GetArrayItem` _waves _waveindex)))
  (bind (_projectedlocation _returnvalue) (`NavigationSystemV1.K2_ProjectPointToNavigation` (`KismetMathLibrary.TransformLocation` (`self.GetTransform`) (`|GetArrayItem` _spawnlocations (mod (`self.SpawnIndex`) (`KismetArrayLibrary.Array_Length` _spawnlocations)))) null null (100.0 100.0 500.0)))
  (if (`KismetArrayLibrary.Array_IsValidIndex` _waves _waveindex)
    (if (`KismetArrayLibrary.Array_IsValidIndex` _enemiesinwave _spawnindex)
      (if _returnvalue
        (bind _returnvalue_2 (`AIBlueprintHelperLibrary.SpawnAIFromClass` (`|GetArrayItem` _enemiesinwave _spawnindex) null (+ _projectedlocation (0.0 0.0 100.0))))
        (`/Engine/EditorBlueprintResources/StandardMacros.IncrementInt` (`self.SpawnIndex`)
          (:`  `
            (`/Engine/EditorBlueprintResources/StandardMacros.IsValid` _returnvalue_2
              (:`Is Valid`
                (`KismetArrayLibrary.Array_Add` (`self.ActiveEnemies`) (cast `/Game/Blueprints/Enemy/BaseEnemyCharacter` _returnvalue_2 :!pure true))
                (add `self.OnDestroyed` _returnvalue_2 (delegate `EnemyDestroyed`))
                (bind _returnvalue_3 (`KismetSystemLibrary.K2_SetTimerDelegate` (`|CreateDelegate` :!event `SpawnNextEnemy`) (`KismetMathLibrary.RandomFloatInRange` _minspawninterval _maxspawninterval)))
                (set `self.NextSpawnTimer` _returnvalue_3))
              (:`Is Not Valid`
                (`self.PrintDebug` "Failed to spawn"
                  (:`Out`
                    (`self.SpawnNextEnemy`)))))))
        (else
          (`self.PrintDebug` "Failed to resolve spawn location on nav graph"))))))

(event `EnemyDestroyed` :!signature `self.OnDestroyed`
  (params (DestroyedActor :type "Actor Object Reference"))
  (bind _asbase_enemy_character (cast `/Game/Blueprints/Enemy/BaseEnemyCharacter` DestroyedActor))
  (`KismetArrayLibrary.Array_RemoveItem` (`self.ActiveEnemies`) _asbase_enemy_character)
  (`self.CheckForClear`))

(fn `UserConstructionScript`)