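; PickupSpawner is a world actor that spawns a configurable pickup at its own transform when flag conditions are met.
; It attempts a spawn on BeginPlay and whenever GameModeBP flags change, resolving required and blocking flags and allowing only one active pickup.
; It passes PickupFlag to the spawned actor.
; OnReset destroys the active pickup, then retries spawning if RespawnOnWorldReset is set.
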(event `self.ReceiveBeginPlay`
  (bind _asgame_mode_bp (cast `/Game/Blueprints/GameModeBP` (`GameplayStatics.GetGameMode`)))
  (add `/Game/Blueprints/GameModeBP.OnGameModeFlagChanged` _asgame_mode_bp (delegate `OnFlagsChanged`))
  (`self.TrySpawn`))

(event `OnFlagsChanged`
  (`self.TrySpawn`))

(event `self.K2_OnReset`
  (bind _activepickup (`self.ActivePickup`))
  (`|ExecutionSequence`
    (:`then_0`
      (`/Engine/EditorBlueprintResources/StandardMacros.IsValid` _activepickup
        (:`Is Valid`
          (`self.K2_DestroyActor` _activepickup))))
    (:`then_1`
      (if (`self.RespawnOnWorldReset`)
        (`self.TrySpawn`)))))

(event `TrySpawn`
  (`/Engine/EditorBlueprintResources/StandardMacros.IsValid` (`self.ActivePickup`)
    (:`Is Not Valid`
      (bind _resolve (`/Game/Blueprints/GameHelperFunctions.ResolveFlags` (`self.RequiredFlags`) (`self.BlockingFlags`)))
      (if _resolve
        (bind _returnvalue (`|SpawnActorFromClass` (`self.PickupClass`) (`self.GetTransform`) "Undefined" "OverrideRootScale" null (`self.PickupFlag`) null))
        (set `self.ActivePickup` _returnvalue)))))

(fn `UserConstructionScript`)