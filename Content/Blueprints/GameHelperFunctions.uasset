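; GameHelperFunctions is a set of helper functions for setting and querying enum-keyed boolean flags stored in a map on GameModeBP.
; SetGameModeFlag writes a value and, when it changes, calls the game mode's change notification and prints a debug message.
; IsGameModeFlagSet reads a flag, returning false if the cast fails.
; ResolveFlags uses it to check that all required flags are set and no blocking flag is.
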(fn `IsGameModeFlagSet`
  (params (GameModeFlag :type "/Game/Blueprints/GameModeFlags Enum" :default "NewEnumerator0"))
  (returns (IsFlagSet :type Boolean))
  (bind _asgame_mode_bp (cast `/Game/Blueprints/GameModeBP` (`GameplayStatics.GetGameMode` (`local.__WorldContext`)))
    (:`then`
      (return (`BlueprintMapLibrary.Map_Find` (`/Game/Blueprints/GameModeBP.GameModeFlagset` _asgame_mode_bp) GameModeFlag)))
    (:`CastFailed`
      (return false))))

(fn `ResolveFlags`
  (params (Required :type "Array of /Game/Blueprints/GameModeFlags Enum") (Blocking :type "Array of /Game/Blueprints/GameModeFlags Enum"))
  (returns (Resolve :type Boolean))
  (for _array_element Required
    (if (not (`self.IsGameModeFlagSet` _array_element (`local.__WorldContext`)))
      (return false)))
  (for _array_element_2 Blocking
    (if (`self.IsGameModeFlagSet` _array_element_2 (`local.__WorldContext`))
      (return false)))
  (return true))

(fn `SetGameModeFlag`
  (params (GameModeFlag :type "/Game/Blueprints/GameModeFlags Enum" :default "NewEnumerator0") (NewValue :type Boolean))
  (locals (OldValue :type Boolean))
  (bind _newvalue (`local.NewValue`))
  (bind _asgame_mode_bp (cast `/Game/Blueprints/GameModeBP` (`GameplayStatics.GetGameMode` (`local.__WorldContext`))))
  (bind _gamemodeflagset (`/Game/Blueprints/GameModeBP.GameModeFlagset` _asgame_mode_bp))
  (bind (_value _returnvalue) (`BlueprintMapLibrary.Map_Find` _gamemodeflagset GameModeFlag))
  (set `local.OldValue` (and _value _returnvalue))
  (`BlueprintMapLibrary.Map_Add` _gamemodeflagset GameModeFlag _newvalue)
  (if (!= _newvalue (`local.OldValue`))
    (`/Game/Blueprints/GameModeBP.OnGameModeFlagChanged` _asgame_mode_bp)
    (`KismetSystemLibrary.PrintText` (`local.__WorldContext`) (`|FormatText` "{0} {1}" (`KismetTextLibrary.Conv_StringToText` (`|GetEnumeratorNameAsString` (`local.GameModeFlag`))) (select `bool` (`local.NewValue`) :`false` "CLEARED" :`true` "SET" :!type "Text")) true true (struct :`R` 0.033124 :`G` 0.677083 :`A` 1.0) 10.0)))