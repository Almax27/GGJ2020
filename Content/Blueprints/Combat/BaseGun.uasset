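; BaseGun is a base weapon actor that fires projectiles automatically while an attack is held.
; BeginAttack and EndAttack toggle firing, while Tick enforces the shot interval and spends ammo.
; An empty clip starts a reload timer on the next shot attempt, with empty BeginReload and EndReload events as hooks.
; FireProjectile spawns the configured projectile class at the gun's transform with an attached sound, or prints a warning if none is set.
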(event `self.ReceiveBeginPlay`
  (set `self.AmmoRemaining` (`self.ClipSize`)))

(event `self.BeginAttack`
  (set `self.IsFiring` true))

(event `self.EndAttack`
  (set `self.IsFiring` false))

(event `self.ReceiveTick`
  (params (DeltaSeconds :type "Float (single-precision)"))
  (if (`self.IsFiring`)
    (if (> (`KismetSystemLibrary.GetGameTimeInSeconds`) (+ (`self.LastFireTime`) (`self.ShotInterval`)))
      (if (> (`self.AmmoRemaining`) 0)
        (`/Engine/EditorBlueprintResources/StandardMacros.DecrementInt` (`self.AmmoRemaining`)
          (:`  `
            (`self.FireProjectile`)))
        (elif (not (`KismetSystemLibrary.K2_IsTimerActiveHandle` (`self.ReloadTimer`)))
          (bind _returnvalue (`KismetSystemLibrary.K2_SetTimerDelegate` (delegate `OnReloadTimerEnd`) (`self.ReloadTime`)))
          (set `self.ReloadTimer` _returnvalue)
          (`self.BeginReload`))))))

(event `OnReloadTimerEnd`
  (set `self.AmmoRemaining` (`self.ClipSize`))
  (`self.EndReload`))

(event `FireProjectile`
  (if (`KismetSystemLibrary.IsValidClass` (`self.ProjectileClass`))
    (`|SpawnActorFromClass` (`self.ProjectileClass`) (`KismetMathLibrary.MakeTransform` (`self.K2_GetActorLocation`) (`self.K2_GetActorRotation`)) "AlwaysSpawn" "OverrideRootScale" (`self.GetOwner`) null (`self.GetInstigator`))
    (`GameplayStatics.SpawnSoundAttached` "/Game/Audio/Weapons/Default_Gun_Fire_00_Cue.Default_Gun_Fire_00_Cue" (`self.DefaultSceneRoot`) "None" (0.0 0.0 0.0) (struct) "KeepRelativeOffset" false 1.0 1.0 0.0 null null)
    (set `self.LastFireTime` (`KismetSystemLibrary.GetGameTimeInSeconds`))
    (else
      (`KismetSystemLibrary.PrintText` (`|FormatText` "{0} has no projectile class set" (`KismetTextLibrary.Conv_StringToText` (`KismetSystemLibrary.GetObjectName` self)))))))

(event `BeginReload`)

(event `EndReload`)

(fn `UserConstructionScript`
  (`parent.UserConstructionScript`))