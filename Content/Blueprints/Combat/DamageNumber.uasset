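; Actor that displays a floating damage number through a widget component, then removes itself.
; On BeginPlay it casts the component's widget to DamageNumberWidget and sets its text to the rounded DamageValue.
; It then plays the widget's Damage animation and destroys the actor when that animation finishes.
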(event `self.ReceiveBeginPlay`
  (bind _asdamage_number_widget (cast `/Game/Blueprints/UI/DamageNumberWidget` (`WidgetComponent.GetUserWidgetObject` (`self.Widget`))))
  (`TextBlock.SetText` (`/Game/Blueprints/UI/DamageNumberWidget.NumberText` _asdamage_number_widget) (`|FormatText` "{0}" (`KismetMathLibrary.Round` (`self.DamageValue`))))
  (`|PlayAnimation` _asdamage_number_widget (`/Game/Blueprints/UI/DamageNumberWidget.Damage` _asdamage_number_widget)
    (:`Finished`
      (`self.K2_DestroyActor`))))

(fn `UserConstructionScript`)