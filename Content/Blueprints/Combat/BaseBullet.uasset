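; Base projectile that homes on enemy characters, applies damage to what it hits and destroys itself.
; On BeginPlay it and its owner ignore each other's movement collision.
; Each tick, GetBestTarget overlaps a homing sphere and picks the lowest squared distance times facing dot, filtered by angle and line of sight, to steer ProjectileMovement.
; Hits play impact sounds chosen for player, enemy or other actors.
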(event `self.ReceiveBeginPlay`
  (bind _asprimitive_component (cast `PrimitiveComponent` (`Actor.RootComponent` (`self.GetOwner`))))
  (`PrimitiveComponent.IgnoreActorWhenMoving` _asprimitive_component self true)
  (`PrimitiveComponent.IgnoreActorWhenMoving` (`self.BulletCollision`) (`self.GetOwner`) true))

(event `self.ReceiveHit`
  (params (MyComp :type "PrimitiveComponent Object Reference") (Other :type "Actor Object Reference") (OtherComp :type "PrimitiveComponent Object Reference") (bSelfMoved :type Boolean) (HitLocation :type "Vector Structure") (HitNormal :type "Vector Structure") (NormalImpulse :type "Vector Structure") (Hit :type "HitResult Structure (by ref)"))
  (`|ExecutionSequence`
    (:`then_0`
      (`GameplayStatics.ApplyDamage` Other (`self.Damage`) (`self.GetInstigatorController`) self (`self.DamageType`)))
    (:`then_1`
      (`self.ProcessHitSound` Other HitLocation))
    (:`then_2`
      (`self.K2_DestroyActor`))))

(event `self.ReceiveTick`
  (params (DeltaSeconds :type "Float (single-precision)"))
  (bind _target (`self.GetBestTarget`))
  (`/Engine/EditorBlueprintResources/StandardMacros.IsValid` _target
    (:`Is Valid`
      (set `ProjectileMovementComponent.HomingTargetComponent` (`Actor.RootComponent` _target) (`self.ProjectileMovement`)))))

(event `ProcessHitSound`
  (params (Actor :type "Actor Object Reference") (HitLocation :type "Vector Structure"))
  (cast `/Game/Blueprints/Player/PlayerCharacter` Actor ; Hit player?
    (:`then`
      (`GameplayStatics.SpawnSoundAtLocation` "/Game/Audio/Weapons/BulletImpact_Metal_Heavy_00_Cue.BulletImpact_Metal_Heavy_00_Cue" HitLocation (struct) 1.0 1.0 0.0 null null))
    (:`CastFailed`
      (cast `/Game/Blueprints/Enemy/BaseEnemyCharacter` Actor ; Hit Enemy?
        (:`then`
          (`GameplayStatics.SpawnSoundAtLocation` "/Game/Audio/Weapons/BulletImpact_Flesh_00_Cue.BulletImpact_Flesh_00_Cue" HitLocation (struct) 1.0 1.0 0.0 null null))
        (:`CastFailed`
          (`GameplayStatics.SpawnSoundAtLocation` "/Game/Audio/Weapons/BulletImpact_Metal_Light_00_Cue.BulletImpact_Metal_Light_00_Cue" HitLocation (struct) 1.0 1.0 0.0 null null))))))

(fn `GetBestTarget`
  (returns (Target :type "Actor Object Reference"))
  (locals (BestTarget :type "Actor Object Reference") (BestWeight :type "Float (double-precision)" :default 1000000000.0) (BulletForward :type "Vector Structure") (BulletLocation :type "Vector Structure") (Weight :type "Float (double-precision)" :default 1000000000.0) (PotentialTarget :type "Actor Object Reference"))
  (bind _potentialtarget (`local.PotentialTarget`))
  (`|ExecutionSequence`
    (:`then_0`
      (set `local.BulletForward` (`self.GetActorForwardVector`))
      (set `local.BulletLocation` (`self.K2_GetActorLocation`)))
    (:`then_1`
      (bind _outactors (`KismetSystemLibrary.SphereOverlapActors` (`self.K2_GetActorLocation`) (`self.HomingRadius`) (`|MakeArray` "ObjectTypeQuery3" :!type "EObjectTypeQuery Enum") "/Game/Blueprints/Enemy/BaseEnemyCharacter.BaseEnemyCharacter_C" (`|MakeArray` (`self.GetOwner`))))
      (for _array_element _outactors
        (bind _output_get (set `local.PotentialTarget` _array_element))
        (bind _returnvalue (- (`self.K2_GetActorLocation` _output_get) (`local.BulletLocation`)))
        (bind _returnvalue_2 (`KismetMathLibrary.Dot_VectorVector` (`KismetMathLibrary.Normal` _returnvalue) (`local.BulletForward`)))
        (bind _returnvalue_3 (* (`KismetMathLibrary.VSizeSquared` _returnvalue) _returnvalue_2))
        (set `local.Weight` _returnvalue_3)
        (if (< _returnvalue_3 (`local.BestWeight`))
          (if (< (`KismetMathLibrary.DegAcos` _returnvalue_2) (`self.HomingAngle`))
            (bind (_outhit _returnvalue_4) (`KismetSystemLibrary.LineTraceSingle` (`local.BulletLocation`) (`self.K2_GetActorLocation` _potentialtarget) "TraceTypeQuery1" true (`|MakeArray` _potentialtarget self :!type "Actor Object Reference") "ForOneFrame"))
            (if (not _returnvalue_4)
              (set `local.BestTarget` (`local.PotentialTarget`))
              (set `local.BestWeight` (`local.Weight`))))))
      (return (`local.BestTarget`)))))

(fn `UserConstructionScript`)