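; CombatComponent is an actor component that tracks health and death for its owner.
; It starts at max health, binds the owner's damage events, and handles only any-damage: recording hit time, subtracting damage and broadcasting health-change and death events.
; The point and radial handlers are empty, and damage-number spawning is disconnected.
; Helper functions report time since last hit and alive state, or kill the owner outright by zeroing health and firing both events.
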(event `self.ReceiveBeginPlay`
  (bind _returnvalue (`self.GetOwner`))
  (set `self.Health` (`self.MaxHealth`))
  (add `Actor.OnTakePointDamage` _returnvalue (`|CreateDelegate` :!event `OnPointDamage`))
  (add `Actor.OnTakeRadialDamage` _returnvalue (`|CreateDelegate` :!event `OnRadialDamage`))
  (add `Actor.OnTakeAnyDamage` _returnvalue (`|CreateDelegate` :!event `OnAnyDamage`)))

(event `OnAnyDamage`
  (params (DamagedActor :type "Actor Object Reference") (Damage :type "Float (double-precision)") (DamageType :type "DamageType Object Reference") (InstigatedBy :type "Controller Object Reference") (DamageCauser :type "Actor Object Reference"))
  (bind _returnvalue (- (`self.Health`) Damage))
  (set `self.LastHitTime` (`KismetSystemLibrary.GetGameTimeInSeconds`))
  (`|ExecutionSequence`
    (:`then_0`
      (if (!= (`KismetMathLibrary.FMax` _returnvalue) (`self.Health`))
        (bind _output_get (set `self.Health` _returnvalue))
        (`self.OnHealthChanaged` self _output_get)))
    (:`then_1`)
    (:`then_2`
      ;[1 1 1] Death
      (if (<= (`self.Health`) 0.0)
        (`self.OnDeath` self)))))

(event `OnPointDamage`
  (params (DamagedActor :type "Actor Object Reference") (Damage :type "Float (double-precision)") (InstigatedBy :type "Controller Object Reference") (HitLocation :type "Vector Structure") (FHitComponent :type "PrimitiveComponent Object Reference") (BoneName :type Name) (ShotFromDirection :type "Vector Structure") (DamageType :type "DamageType Object Reference") (DamageCauser :type "Actor Object Reference")))

(event `OnRadialDamage`
  (params (DamagedActor :type "Actor Object Reference") (Damage :type "Float (double-precision)") (DamageType :type "DamageType Object Reference") (Origin :type "Vector Structure") (HitInfo :type "HitResult Structure") (InstigatedBy :type "Controller Object Reference") (DamageCauser :type "Actor Object Reference")))

(event `self.ReceiveEndPlay`
  (params (EndPlayReason :type "EEndPlayReason Enum" :default "Destroyed")))

(fn `GetTimeSinceLastHit`
  (returns (Seconds :type "Float (double-precision)"))
  (return (- (`KismetSystemLibrary.GetGameTimeInSeconds`) (`self.LastHitTime`))))

(fn `IsAlive`
  (returns (IsAlive :type Boolean))
  (return (> (`self.Health`) 0.0)))

(fn `Kill`
  (bind _output_get (set `self.Health` 0.0))
  (`self.OnHealthChanaged` self _output_get)
  (`self.OnDeath` self))